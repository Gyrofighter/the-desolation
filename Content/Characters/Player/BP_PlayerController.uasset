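; Player controller that relays player feedback to the HUD and handles the pause menu, camera shakes and mouse sensitivity.
; On BeginPlay it reads sensitivity from the game instance and applies it to both pitch and yaw input scales.
; Damage and saving notices go to the HUD through message calls, while the pause menu casts to BP_HUD.
; The Menu input skips an active cinematic via the game mode, otherwise it opens the pause menu.
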(event EventChangeMouseSensitivity
  (params (Sensitivity :type Float%20%28single-precision%29))
  ;[1 1 1] MouseSensitivity
  (Variables|Default|SetInputPitchScale Sensitivity)
  (Variables|Default|SetInputYawScale Sensitivity))

(event EventBeginPlay
  ;[1 1 1] BeginPlay
  (bind _sensitivity (Class|GameInstanceInterface|GetMouseSensitivity(Message) (Game|GetGameInstance)))
  (CallFunction|ChangeMouseSensitivity _sensitivity))

(event EventStartCameraShake
  (params (Shake :type Camera%20Shake%20Class%20Reference) (Scale :type Float%20%28single-precision%29))
  ;[1 1 1] CameraShakes
  (Class|PlayerController|ClientPlayCameraShake Shake Scale "CameraLocal" "0, 0, 0"))

(event EventStopCameraShake
  (params (Shake :type Camera%20Shake%20Class%20Reference))
  ;[1 1 1] CameraShakes
  (Game|Feedback|ClientStopCameraShake Shake false))

(event EventPawnDamaged
  ;[1 1 1] PawnDamaged
  (Class|HUDInterface|DamageBloodMask(Message) (HUD|GetHUD)))

(event EventShowPauseMenu
  (params (Text :type Text))
  ;[1 1 1] PauseOnDead
  (bind _asbp_hud (Utilities|Casting|CastToBP_HUD (HUD|GetHUD)))
  (Default|ShowPauseMenu _asbp_hud Text))

(event EventSaving
  ;[1 1 1] Saving
  (Class|HUDInterface|Saving(Message) (HUD|GetHUD)))

(event Input|ActionEvents|InputActionMenu
  (params (Key :type Key%20Structure :default "None"))
  (bind _returnvalue (Game|GetGameMode))
  ;[1 1 1] Pause
  (:Pressed
    (bind _active (Class|GameModeInterface|GetCinematicActive(Message) _returnvalue))
    (if _active
      (Class|GameModeInterface|SkipCinematic(Message) _returnvalue)
      (else
        (CallFunction|ShowPauseMenu "Pause")))))

(fn ConstructionScript)