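; First-person player character with a rifle, grenades, sprint, ironsights and crouch, restored from SaveInfo on BeginPlay.
; A looping timer drives hitscan fire with random spread, headshot multiplier and surface-based impact effects, while montages time reloads and grenade throws.
; State flags gate actions, timelines animate FOV and camera, and the controller receives shake, damage and death messages.
; Damage pauses health regeneration on a delay, and dispatchers broadcast ammo and aim changes.
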(event OnDeath(BP_HealthComponent)
  ;[1 1 1] Death
  (Animation|StopAnimMontage 0)
  (Input|DisableInput 0)
  (CallFunction|StopSoundShooting)
  (Utilities|FlowControl|Delay 2.0)
  (Class|PlayerControllerInterface|ShowPauseMenu(Message) (Pawn|GetController) "You Died"))

(event Custom|Shooting
  (bind _weapon (Variables|Default|GetWeapon))
  ;[1 1 1] Shooting
  (CallFunction|StopSprint)
  (if (CallFunction|CanShoot)
    (if (> (Variables|Weapon|GetBullets) 0)
      (Animation|Montage|PlayMontage (Variables|Default|GetFPSMesh) (CallFunction|GetShootMontage)
        (:then
          (CallFunction|TraceProjectile)
          (Variables|Weapon|SetIsShooting true)
          (CallFunction|EffectsandCamera)
          (Variables|Default|GetShootLoop
            (:then)
            (:else
              (bind _returnvalue (Audio|SpawnSoundAttached "/Game/Sounds/Weapon/SC_WeaponShotLoop.SC_WeaponShotLoop" _weapon "None" (Transformation|GetWorldLocation _weapon) "0, 0, 0" "SnapToTarget" true 1.0 1.0 0.0 "/Game/Sounds/StandartSoundAttenuation.StandartSoundAttenuation" 0))
              (Variables|Default|SetShootLoop _returnvalue))))
        (:OnCompleted
          (Variables|Weapon|SetIsShooting false)
          (if (Variables|Movements|GetIsSprintInputActive)
            (CallFunction|StartSprint)))
        (:OnInterrupted
          (Variables|Weapon|SetIsShooting false)))
      (else
        (CallFunction|Reload)
        (CallFunction|StopSoundShooting)))))

(event Custom|StartSprint
  ;[1 1 1] Sprint
  (if (CallFunction|CanSprint)
    (Variables|/Script/Engine.CharacterMovementComponent|SetMaxWalkSpeed (Variables|Character|GetCharacterMovement) (Variables|Movements|GetSprintSpeed))
    (Variables|Movements|SetIsSprinting true)
    (bind _fov (Timeline|Sprint Play)
      (:Update
        (Camera|SetFieldOfView (Variables|Default|GetCamera) _fov)))))

(event Custom|StopSprint
  ;[1 1 1] Sprint
  (if (Variables|Movements|GetIsSprinting)
    (Variables|/Script/Engine.CharacterMovementComponent|SetMaxWalkSpeed (Variables|Character|GetCharacterMovement) (Variables|Movements|GetWalkSpeed))
    (Utilities|FlowControl|Delay 0.25)
    (Variables|Movements|SetIsSprinting false)
    (bind _fov (Timeline|Sprint Reverse)
      (:Update
        (Camera|SetFieldOfView (Variables|Default|GetCamera) _fov)))))

(event Custom|StartIronsight
  (bind _startmeshposition (Variables|Other|GetStartMeshPosition))
  ;[1 1 1] Ironsight
  (if (Math|Boolean|ANDBoolean (Variables|Weapon|GetIsSecondaryFireActive) (not (Variables|Movements|GetIsSprinting)) (not (Variables|Weapon|GetIsReloading)))
    (Variables|Weapon|SetisIronsight true)
    (Default|CallOnStartIronSight)
    (Variables|/Script/Engine.CharacterMovementComponent|SetMaxWalkSpeed (Variables|Character|GetCharacterMovement) (Variables|Weapon|GetIronsightSpeed))
    (Components|Timeline|SetPlayRate (Variables|Default|GetIronSightTimeline) 4.0)
    (bind _ironsight (Timeline|IronSightTimeline Play)
      (:Update
        (Camera|SetFieldOfView (Variables|Default|GetCamera) (Math|Float|Lerp 9e+01 5e+01 _ironsight))
        (Transformation|SetRelativeLocation (Variables|Default|GetFPSMesh) (Math|Vector|Lerp(Vector) _startmeshposition (+ _startmeshposition "-55.000000,0.000000,-0.250000") _ironsight) false false)))))

(event Custom|StopIronsight
  (bind _startmeshposition (Variables|Other|GetStartMeshPosition))
  ;[1 1 1] Ironsight
  (if (Variables|Weapon|GetisIronsight)
    (Variables|Weapon|SetisIronsight false)
    (Default|CallOnEndIronSight)
    (Variables|/Script/Engine.CharacterMovementComponent|SetMaxWalkSpeed (Variables|Character|GetCharacterMovement) (Variables|Movements|GetWalkSpeed))
    (Components|Timeline|SetPlayRate (Variables|Default|GetIronSightTimeline) 4.0)
    (bind _ironsight (Timeline|IronSightTimeline Reverse)
      (:Update
        (Camera|SetFieldOfView (Variables|Default|GetCamera) (Math|Float|Lerp 9e+01 5e+01 _ironsight))
        (Transformation|SetRelativeLocation (Variables|Default|GetFPSMesh) (Math|Vector|Lerp(Vector) _startmeshposition (+ _startmeshposition "-55.000000,0.000000,-0.250000") _ironsight) false false)))))

(event Custom|Reload
  ;[1 1 1] Reload
  (if (CallFunction|CanReload)
    (Animation|Montage|PlayMontage (Variables|Default|GetWeapon) "/Game/Characters/Player/Animations/Weapon/A_Rifle_Reload_Montage.A_Rifle_Reload_Montage"
      (:then
        (Animation|Montage|PlayMontage (Variables|Default|GetFPSMesh) "/Game/Characters/Player/Animations/A_Reload_Montage.A_Reload_Montage"
          (:then
            (Variables|Weapon|SetIsReloading true)
            (Audio|PlaySoundatLocation "/Game/Sounds/Weapon/SC_Weapon_Reload.SC_Weapon_Reload" "0, 0, 0" "0, 0, 0" 1.0 1.0 0.0 0 0 0)
            (CallFunction|StartCameraShake "/Game/Characters/Player/CameraShakes/ReloadCameraShake.ReloadCameraShake_C" 1.0)
            (CallFunction|StopSprint))
          (:OnInterrupted
            (Variables|Weapon|SetIsReloading false)
            (CallFunction|StopCameraShake "/Game/Characters/Player/CameraShakes/ReloadCameraShake.ReloadCameraShake_C" :!label _label))
          (:OnNotifyEnd
            (Variables|Weapon|SetIsReloading false)
            (bind _output_get (Variables|Weapon|SetBullets (Variables|Weapon|GetMaxBullets)))
            (Default|CallOnBulletsChange _output_get)
            (goto _label)))))))

(event Custom|StartRegen
  ;[1 1 1] AnyDamage/Regen
  (if (Variables|Other|GetCanRegenHP)
    (Variables|/Game/Base/Components/BP_HealthComponent.BP_HealthComponent_C|SetHealthPerSecond (Variables|Default|GetBP_HealthComponent) 1e+01)))

(event Game|Damage|EventAnyDamage
  (params (Damage :type Float%20%28single-precision%29) (DamageType :type Damage%20Type%20Object%20Reference) (InstigatedBy :type Controller%20Object%20Reference) (DamageCauser :type Actor%20Object%20Reference))
  ;[1 1 1] AnyDamage/Regen
  (|CallParentFunction Damage DamageType InstigatedBy DamageCauser)
  (Variables|/Game/Base/Components/BP_HealthComponent.BP_HealthComponent_C|SetHealthPerSecond (Variables|Default|GetBP_HealthComponent) 0.0)
  (Utilities|Time|SetTimerbyFunctionName 0 "StartRegen" 1e+01)
  (CallFunction|StartCameraShake "/Game/Characters/Player/CameraShakes/DamageCameraShake.DamageCameraShake_C" (Math|Float|Min(Float) 5.0 (/ Damage 5.0)))
  (Class|PlayerControllerInterface|PawnDamaged(Message) (Pawn|GetController)))

(event EventOnEndCrouch
  (params (HalfHeightAdjust :type Float%20%28single-precision%29) (ScaledHalfHeightAdjust :type Float%20%28single-precision%29))
  (bind _startcameraposition (Variables|Other|GetStartCameraPosition))
  ;[1 1 1] CrouchAdd
  (CallFunction|StartCameraShake "/Game/Characters/Player/CameraShakes/CrouchCameraShake.CrouchCameraShake_C" 1.0)
  (bind _alpha (Timeline|CrouchTimeline Reverse)
    (:Update
      (Transformation|SetRelativeLocation (Variables|Default|GetCamera) (Math|Vector|MakeVector (.x _startcameraposition) (.y _startcameraposition) (+ (.z _startcameraposition) _alpha)) false false))))

(event EventOnStartCrouch
  (params (HalfHeightAdjust :type Float%20%28single-precision%29) (ScaledHalfHeightAdjust :type Float%20%28single-precision%29))
  (bind _startcameraposition (Variables|Other|GetStartCameraPosition))
  ;[1 1 1] CrouchAdd
  (CallFunction|StartCameraShake "/Game/Characters/Player/CameraShakes/CrouchCameraShake.CrouchCameraShake_C" 1.0)
  (bind _alpha (Timeline|CrouchTimeline Play)
    (:Update
      (Transformation|SetRelativeLocation (Variables|Default|GetCamera) (Math|Vector|MakeVector (.x _startcameraposition) (.y _startcameraposition) (+ (.z _startcameraposition) _alpha)) false false))))

(event EventTick
  (params (DeltaSeconds :type Float%20%28single-precision%29))
  ;[1 1 1] Tick
  (CallFunction|CameraShake)
  (CallFunction|CheckSprint))

(event EventOnLanded
  (params (Hit :type Hit%20Result%20Structure%20%28by%20ref%29))
  ;[1 1 1] JumpCameraShake
  (CallFunction|StartCameraShake "/Game/Characters/Player/CameraShakes/JumpCameraShake.JumpCameraShake_C" (/ (Math|Float|Absolute(Float) (.z (Transformation|GetVelocity))) 4e+02)))

(event EventOnJumped
  ;[1 1 1] JumpCameraShake
  (CallFunction|StartCameraShake "/Game/Characters/Player/CameraShakes/JumpCameraShake.JumpCameraShake_C" 1.0))

(event EventBeginPlay
  ;[1 1 1] BeginPlay
  (CallFunction|LoadData))

(event EventDarkCameraStart
  ;[1 1 1] DarkCamera
  (CallFunction|StartCameraShake "/Game/Characters/Player/CameraShakes/DarkCameraShake.DarkCameraShake_C" 1.0)
  (bind _exp (Timeline|DarkCameraTimeline PlayFromStart)
    (:Update
      (Variables|/Script/Engine.CameraComponent|SetPostProcessSettings (Variables|Default|GetCamera) (Utilities|Struct|MakePostProcessSettings _exp)))))

(event Input|ActionEvents|InputActionJump
  (params (Key :type Key%20Structure :default "None"))
  ;[1 1 1] BasicContols
  (:Pressed
    (Character|Jump))
  (:Released
    (Character|StopJumping)))

(event Input|ActionEvents|InputActionPrimaryFire
  (params (Key :type Key%20Structure :default "None"))
  ;[1 1 1] Shooting
  (:Pressed
    (CallFunction|Shooting)
    (bind _returnvalue (Utilities|Time|SetTimerbyEvent (delegate Custom|Shooting) (/ 1.0 (Variables|Weapon|GetShotsPerSecond)) true))
    (Variables|Weapon|SetShootTimer _returnvalue))
  (:Released
    (Utilities|Time|ClearandInvalidateTimerbyHandle (Variables|Weapon|GetShootTimer))
    (CallFunction|StopSoundShooting)))

(event Input|ActionEvents|InputActionSprint
  (params (Key :type Key%20Structure :default "None"))
  ;[1 1 1] Sprint
  (:Pressed
    (Variables|Movements|SetIsSprintInputActive true)
    (CallFunction|StartSprint))
  (:Released
    (Variables|Movements|SetIsSprintInputActive false)
    (CallFunction|StopSprint)))

(event Input|ActionEvents|InputActionCrouch
  (params (Key :type Key%20Structure :default "None"))
  ;[1 1 1] CrochBasic
  (:Pressed
    (Character|Crouch))
  (:Released
    (Character|UnCrouch)))

(event Input|ActionEvents|InputActionReload
  (params (Key :type Key%20Structure :default "None"))
  ;[1 1 1] Reload
  (:Pressed
    (CallFunction|Reload)))

(event Input|ActionEvents|InputActionSecondaryFire
  (params (Key :type Key%20Structure :default "None"))
  ;[1 1 1] Ironsight
  (:Pressed
    (Variables|Weapon|SetIsSecondaryFireActive true)
    (CallFunction|StartIronsight))
  (:Released
    (Variables|Weapon|SetIsSecondaryFireActive false)
    (CallFunction|StopIronsight)))

(event Input|ActionEvents|InputActionGrenade
  (params (Key :type Key%20Structure :default "None"))
  ;[1 1 1] LaunchGrenade
  (:Pressed
    (if (CallFunction|CanLaunchGrenade)
      (bind _notifyname (Animation|Montage|PlayMontage (Variables|Default|GetFPSMesh) "/Game/Characters/Player/Animations/A_Grenade_Montage.A_Grenade_Montage")
        (:then
          (Variables|Weapon|SetIsLaunchingGrenade true)
          (CallFunction|StartCameraShake "/Game/Characters/Player/CameraShakes/GrenadeCameraShake.GrenadeCameraShake_C" 1.0))
        (:OnInterrupted
          (Variables|Weapon|SetIsLaunchingGrenade false :!label _label))
        (:OnNotifyBegin
          (if (Utilities|Name|Equal(Name) _notifyname "Launch")
            (CallFunction|SpawnGrenade)))
        (:OnNotifyEnd
          (goto _label))))))

(event Input|AxisEvents|InputAxisMoveForward
  (params (AxisValue :type Float%20%28single-precision%29))
  ;[1 1 1] BasicContols
  (Pawn|Input|AddMovementInput (Transformation|GetActorForwardVector) AxisValue false))

(event Input|AxisEvents|InputAxisMoveLeft
  (params (AxisValue :type Float%20%28single-precision%29))
  ;[1 1 1] BasicContols
  (Pawn|Input|AddMovementInput (Transformation|GetActorRightVector) AxisValue false))

(event Input|AxisEvents|InputAxisLookX
  (params (AxisValue :type Float%20%28single-precision%29))
  ;[1 1 1] BasicContols
  (Pawn|Input|AddControllerYawInput AxisValue))

(event Input|AxisEvents|InputAxisLookY
  (params (AxisValue :type Float%20%28single-precision%29))
  ;[1 1 1] BasicContols
  (Pawn|Input|AddControllerPitchInput AxisValue))

(fn ConstructionScript
  (|CallParentFunction)
  (Variables|/Script/Engine.CharacterMovementComponent|SetMaxWalkSpeed (Variables|Character|GetCharacterMovement) (Variables|Movements|GetWalkSpeed))
  (Variables|Other|SetStartCameraPosition (Variables|/Script/Engine.SceneComponent|GetRelativeLocation (Variables|Default|GetCamera)))
  (Variables|Other|SetStartMeshPosition (Variables|/Script/Engine.SceneComponent|GetRelativeLocation (Variables|Default|GetFPSMesh))))

(fn GetShootMontage
  (bind _isightshootmontages (Variables|Animation|GetISightShootMontages))
  (bind _walkshootmontages (Variables|Animation|GetWalkShootMontages))
  (return (select (Variables|Weapon|GetisIronsight) (Utilities|Array|Get(acopy) _isightshootmontages (Math|Random|RandomInteger (Utilities|Array|Length _isightshootmontages))) (Utilities|Array|Get(acopy) _walkshootmontages (Math|Random|RandomInteger (Utilities|Array|Length _walkshootmontages))))))

(fn TraceProjectile
  (bind _camera (Variables|Default|GetCamera))
  (bind _returnvalue (Transformation|GetWorldLocation _camera))
  (bind _result (Math|Integer|DecrementInt (Variables|Weapon|GetBullets))
    (:%20%20
      (Default|CallOnBulletsChange _result)
      (Class|PawnNoiseEmitterComponent|MakeNoise (Variables|Default|GetPawnNoiseEmitter) self 1.0 (Transformation|GetActorLocation))
      (bind (_outhit _returnvalue_2) (Collision|LineTraceByChannel _returnvalue (+ _returnvalue (* (Math|Vector|GetForwardVector _camera) (Variables|Weapon|GetShootRange)) (CallFunction|GetShootingCalibration)) "TraceTypeQuery3" false 0 "None"))
      (if _returnvalue_2
        (CallFunction|AddImpulseforPhysics (.hitcomponent _outhit) (Math|Vector|Normalize (- (.tracestart _outhit) (.traceend _outhit))) (.location _outhit))
        (Effects|SpawnEmitterAttached (.Emitter (CallFunction|GetEmitterbyPhysMat (.physmat _outhit))) (.hitcomponent _outhit) "None" (.location _outhit) (Math|Conversions|RotationFromXVector (.normal _outhit)) (.EmitterScale (CallFunction|GetEmitterbyPhysMat (.physmat _outhit))) "KeepWorldPosition")
        (Audio|PlaySoundatLocation (.Sound (CallFunction|GetEmitterbyPhysMat (.physmat _outhit))) (.location _outhit) "0, 0, 0" 1.0 1.0 0.0 "/Game/Sounds/StandartSoundAttenuation.StandartSoundAttenuation" 0 0)
        (Class|GameplayStatics|SpawnDecalAttached (.Material (CallFunction|GetDecalMatbyPhysMat (.physmat _outhit))) (.DecalSize (CallFunction|GetDecalMatbyPhysMat (.physmat _outhit))) (.hitcomponent _outhit) "None" (.location _outhit) (Math|Rotator|MakeRotator (Math|Random|RandomFloatinRange -1.8e+02 1.8e+02) (.Pitch (Math|Rotator|BreakRotator (Math|Conversions|RotationFromXVector (.normal _outhit)))) (.Yaw (Math|Rotator|BreakRotator (Math|Conversions|RotationFromXVector (.normal _outhit))))) "KeepWorldPosition" 0.0)
        (Game|Damage|ApplyDamage (.hitactor _outhit) (CallFunction|GetWeaponDamage (.hitbonename _outhit)) (Pawn|GetController) self)
        (return)))))

(fn GetShootingCalibration
  (return (select (Variables|Weapon|GetisIronsight) (* (Math|Random|RandomUnitVector) 1e+01) (* (Math|Random|RandomUnitVector) 5e+01))))

(fn SpawnGrenade
  (Game|SpawnActorfromClass "/Game/Weapon/GrenadeProjectile.GrenadeProjectile_C" (Math|Transform|MakeTransform (Transformation|GetSocketLocation (Variables|Default|GetFPSMesh) "GrenadeSocket") (.rotation (Transformation|GetWorldTransform (Variables|Default|GetCamera))) "1,1,1") "Undefined" 0 self)
  (bind _result (Math|Integer|DecrementInt (Variables|Weapon|GetGrenades))
    (:%20%20
      (Default|CallOnLaunchGrenade _result))))

(fn CanShoot
  (return (Math|Boolean|ANDBoolean (not (Variables|Movements|GetIsSprinting)) (not (Variables|Weapon|GetIsReloading)) (not (Variables|Weapon|GetIsLaunchingGrenade)) (not (Default|GetIsDead (Variables|Default|GetBP_HealthComponent))))))

(fn CanReload
  (return (Math|Boolean|ANDBoolean (not (Variables|Weapon|GetIsShooting)) (not (Variables|Weapon|GetIsReloading)) (!= (Variables|Weapon|GetBullets) (Variables|Weapon|GetMaxBullets)))))

(fn CanLaunchGrenade
  (return (Math|Boolean|ANDBoolean (not (Variables|Weapon|GetIsShooting)) (not (Variables|Weapon|GetIsReloading)) (not (Variables|Weapon|GetIsLaunchingGrenade)) (> (Variables|Weapon|GetGrenades) 0))))

(fn AddImpulseforPhysics
  (params (Target :type Primitive%20Component%20Object%20Reference) (Direction :type Vector) (Location :type Vector))
  (if (Physics|IsSimulatingPhysics Target "None")
    (Physics|AddImpulseatLocation Target (* Direction (Variables|Weapon|GetImpulsePower)) Location "None")))

(fn GetDecalMatbyPhysMat
  (params (PhysMat :type Physical%20Material%20Object%20Reference))
  (bind _surfacetype (Variables|/Script/Engine.PhysicalMaterial|GetSurfaceType PhysMat))
  (bind _returnvalue (Utilities|Select :Index _surfacetype :SurfaceType_Default 5.0 :SurfaceType1 0.0 :SurfaceType2 0.0))
  (bind _returnvalue_2 (Utilities|Select :Index _surfacetype :SurfaceType_Default 2.0 :SurfaceType1 0.0 :SurfaceType2 0.0))
  (bind _returnvalue_3 (Math|Random|RandomFloatinRange _returnvalue_2 _returnvalue))
  (return (Utilities|Select :Index _surfacetype :SurfaceType_Default "/Game/Effects/Decals/Materials/D_BasicDamage.D_BasicDamage" :SurfaceType1 0 :SurfaceType2 0) (Math|Vector|MakeVector 1.0 _returnvalue_3 _returnvalue_3)))

(fn GetWeaponDamage
  (params (BoneName :type Name))
  (if (Utilities|Name|Equal(Name) BoneName "Head")
    (return (* (Variables|Weapon|GetDamage) (Variables|Weapon|GetHeadDamageMultiplier)))
    (else
      (return (Variables|Weapon|GetDamage)))))

(fn StopSoundShooting
  (bind _shootloop (Variables|Default|GetShootLoop)
    (:then
      (Components|DestroyComponent _shootloop)
      (Audio|PlaySoundatLocation "/Game/Sounds/Weapon/SC_WeaponStopLoop.SC_WeaponStopLoop" (Transformation|GetWorldLocation (Variables|Default|GetWeapon)) "0, 0, 0" 1.0 1.0 0.0 0 0 0))
    (:else)))

(fn EffectsandCamera
  (Effects|SpawnEmitterAttached "/Game/Effects/Particles/P_Rifle_Muzzleflash.P_Rifle_Muzzleflash" (Variables|Default|GetWeapon) "MuzzleSocket" "0, 0, 0" "0, 0, 0" "1.000000,1.000000,1.000000" "SnapToTarget")
  (Effects|SpawnEmitterAttached "/Game/Effects/Particles/P_Rifle_ShellEject.P_Rifle_ShellEject" (Variables|Default|GetWeapon) "ShellEjectionSocket" "0, 0, 0" "0, 0, 0" "1.000000,1.000000,1.000000" "SnapToTarget")
  (CallFunction|StartCameraShake "/Game/Characters/Player/CameraShakes/ShootCameraShake.ShootCameraShake_C" (+ (select (Variables|Weapon|GetisIronsight) 0.05 0.6) (select (Variables|Default|GetbIsCrouched) 0.05 0.1) (select (<= (Math|Vector|VectorLength (Transformation|GetVelocity)) 2e+02) 0.05 0.3)))
  (return))

(fn StartCameraShake
  (params (Shake :type Camera%20Shake%20Class%20Reference) (Scale :type Float%20%28single-precision%29))
  (Class|PlayerControllerInterface|StartCameraShake(Message) (Pawn|GetController) Shake Scale))

(fn StopCameraShake
  (params (Shake :type Camera%20Shake%20Class%20Reference))
  (Class|PlayerControllerInterface|StopCameraShake(Message) (Pawn|GetController) Shake))

(fn CameraShake
  (if (and (not (Variables|Weapon|GetisIronsight)) (>= (Math|Vector|VectorLength (Transformation|GetVelocity)) 1e+02))
    (CallFunction|StartCameraShake (select (Variables|Movements|GetIsSprinting) "/Game/Characters/Player/CameraShakes/RunCameraShake.RunCameraShake_C" "/Game/Characters/Player/CameraShakes/WalkCameraShake.WalkCameraShake_C") 1.0)
    (return)))

(fn IsinDanger
  (return false))

(fn CheckSprint
  (if (and (Variables|Movements|GetIsSprinting) (== (+ (Math|Float|Absolute(Float) (Input|AxisValues|GetMoveForward)) (Math|Float|Absolute(Float) (Input|AxisValues|GetMoveLeft))) 0.0))
    (CallFunction|StopSprint))
  (return))

(fn CanSprint
  (return (Math|Boolean|ANDBoolean (Variables|Movements|GetIsSprintInputActive) (not (Variables|Weapon|GetIsShooting)) (not (Variables|Weapon|GetisIronsight)) (not (Variables|Weapon|GetIsReloading)) (>= (Math|Vector|VectorLength (Transformation|GetVelocity)) 2e+02))))

(fn LoadData
  (bind _saveinfo (Variables|Other|GetSaveInfo))
  (bind (_transform _bullets _grenades _health) (Utilities|Struct|BreakSPlayerSaveInfo _saveinfo))
  (Transformation|SetActorTransform _transform)
  (Variables|Weapon|SetBullets _bullets)
  (Variables|Weapon|SetGrenades _grenades)
  (Variables|/Game/Base/Components/BP_HealthComponent.BP_HealthComponent_C|SetHealth (Variables|Default|GetBP_HealthComponent) _health))

(fn RefreshInfo
  (bind _bp_healthcomponent (Variables|Default|GetBP_HealthComponent))
  (Default|CallOnBulletsChange (Variables|Weapon|GetBullets))
  (Default|CallOnLaunchGrenade (Variables|Weapon|GetGrenades))
  (Default|CallOnHealthChanged _bp_healthcomponent (Variables|/Game/Base/Components/BP_HealthComponent.BP_HealthComponent_C|GetHealth _bp_healthcomponent) 0.0))