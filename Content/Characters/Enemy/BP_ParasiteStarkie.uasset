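; Parasite Starkie melee enemy that randomizes its mesh scale and material alpha power on spawn.
; Attack montage notifies enable the matching hand's query collision and raise walk speed and acceleration for a lunge, restoring both when the notify ends.
; A damaging hand overlap disables that hand, plays impact effects and sends a StopAttack AI message.
; Interrupted attacks switch both hands off and restore movement.
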(event OnComponentBeginOverlap(RightHandCollision)
  (params (OverlappedComponent :type Primitive%20Component%20Object%20Reference) (OtherActor :type Actor%20Object%20Reference) (OtherComp :type Primitive%20Component%20Object%20Reference) (OtherBodyIndex :type Integer) (bFromSweep :type Boolean) (SweepResult :type Hit%20Result%20Structure%20%28by%20ref%29))
  (bind _righthandcollision (Variables|Default|GetRightHandCollision))
  (bind _returnvalue (Transformation|GetWorldLocation _righthandcollision))
  ;[1 1 1] DamageActors
  (bind _isdamaged (CallFunction|DamageActor OtherActor))
  (if _isdamaged
    (Collision|SetCollisionEnabled _righthandcollision "NoCollision")
    (Effects|SpawnEmitterAttached "/Game/Effects/Particles/P_body_bullet_impact.P_body_bullet_impact" OtherComp "None" _returnvalue (Transformation|GetWorldRotation _righthandcollision) "1.000000,1.000000,1.000000" "KeepWorldPosition")
    (Audio|PlaySoundatLocation "/Game/Sounds/Impacts/SC_Melee_Hit.SC_Melee_Hit" _returnvalue "0, 0, 0" 1.0 1.0 0.0 0 0 0)
    (Class|AIBlueprintHelperLibrary|SendAIMessage self "StopAttack" 0 true)))

(event OnComponentBeginOverlap(LeftHandCollision)
  (params (OverlappedComponent :type Primitive%20Component%20Object%20Reference) (OtherActor :type Actor%20Object%20Reference) (OtherComp :type Primitive%20Component%20Object%20Reference) (OtherBodyIndex :type Integer) (bFromSweep :type Boolean) (SweepResult :type Hit%20Result%20Structure%20%28by%20ref%29))
  (bind _lefthandcollision (Variables|Default|GetLeftHandCollision))
  (bind _returnvalue (Transformation|GetWorldLocation _lefthandcollision))
  ;[1 1 1] DamageActors
  (bind _isdamaged (CallFunction|DamageActor OtherActor))
  (if _isdamaged
    (Collision|SetCollisionEnabled _lefthandcollision "NoCollision")
    (Effects|SpawnEmitterAttached "/Game/Effects/Particles/P_body_bullet_impact.P_body_bullet_impact" OtherComp "None" _returnvalue (Transformation|GetWorldRotation _lefthandcollision) "1.000000,1.000000,1.000000" "KeepWorldPosition")
    (Audio|PlaySoundatLocation "/Game/Sounds/Impacts/SC_Melee_Hit.SC_Melee_Hit" _returnvalue "0, 0, 0" 1.0 1.0 0.0 0 0 0)
    (Class|AIBlueprintHelperLibrary|SendAIMessage self "StopAttack" 0 true)))

(event EventAttackInterrupted
  (bind _charactermovement (Variables|Character|GetCharacterMovement))
  ;[1 1 1] HandsCollision
  (CallFunction|OffHandCollision)
  (Variables|/Script/Engine.CharacterMovementComponent|SetMaxWalkSpeed _charactermovement (Variables|Default|GetRunSpeed))
  (Variables|/Script/Engine.CharacterMovementComponent|SetMaxAcceleration _charactermovement 2048.0))

(event EventOnNotifyBegin
  (params (NotifyName :type Name :default "None"))
  (bind _charactermovement (Variables|Character|GetCharacterMovement))
  ;[1 1 1] HandsCollision
  (|CallParentFunction NotifyName)
  (CallFunction|SetHandCollision NotifyName "QueryOnly")
  (Variables|/Script/Engine.CharacterMovementComponent|SetMaxWalkSpeed _charactermovement 1e+03)
  (Variables|/Script/Engine.CharacterMovementComponent|SetMaxAcceleration _charactermovement 4096.0))

(event EventOnNotifyEnd
  (params (NotifyName :type Name :default "None"))
  (bind _charactermovement (Variables|Character|GetCharacterMovement))
  ;[1 1 1] HandsCollision
  (|CallParentFunction NotifyName)
  (CallFunction|SetHandCollision NotifyName "NoCollision")
  (Variables|/Script/Engine.CharacterMovementComponent|SetMaxWalkSpeed _charactermovement (Variables|Default|GetRunSpeed))
  (Variables|/Script/Engine.CharacterMovementComponent|SetMaxAcceleration _charactermovement 2048.0))

(event EventBeginPlay
  ;[1 1 1] BeginPlay
  (|CallParentFunction)
  (CallFunction|OffHandCollision)
  (Rendering|Material|SetScalarParameterValueonMaterials (Variables|Character|GetMesh) "AlphaPower" (Math|Random|RandomFloatinRange 0.0 (Variables|Default|GetMatetialAlphaPower)))
  (Transformation|SetRelativeScale3D (Variables|Character|GetMesh) (Math|Conversions|ToVector(Float) (Math|Random|RandomFloatinRange (Variables|Default|GetMinScale) (Variables|Default|GetMaxSale)))))

(fn ConstructionScript
  (|CallParentFunction))

(fn SetHandCollision
  (params (NotifyName :type Name) (CollisionType :type ECollisionEnabled%20Enum :default "NoCollision"))
  (switch name NotifyName
    (:LeftAttack
      (Collision|SetCollisionEnabled (Variables|Default|GetLeftHandCollision) CollisionType))
    (:RightAttack
      (Collision|SetCollisionEnabled (Variables|Default|GetRightHandCollision) CollisionType))))

(fn OffHandCollision
  (Collision|SetCollisionEnabled (Variables|Default|GetRightHandCollision) "NoCollision")
  (Collision|SetCollisionEnabled (Variables|Default|GetLeftHandCollision) "NoCollision"))