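; Enemy ambush trigger box that spawns enemies at placed SpawnActors when the player enters or leaves it.
; Each overlap requires the game mode's player-in-danger flag and passes a weighted chance roll.
; A DoOnce limits it to one ambush, which signals OnTriggered, plays a sound and optionally starts camera darkening and combat music.
; A random count spawns per point, and each enemy immediately sees the player.
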(event OnComponentBeginOverlap(Box)
  (params (OverlappedComponent :type Primitive%20Component%20Object%20Reference) (OtherActor :type Actor%20Object%20Reference) (OtherComp :type Primitive%20Component%20Object%20Reference) (OtherBodyIndex :type Integer) (bFromSweep :type Boolean) (SweepResult :type Hit%20Result%20Structure%20%28by%20ref%29))
  (Utilities|Casting|CastToBP_PlayerCharacter OtherActor)
  (bind _notindanger (Class|GameModeInterface|GetPlayerinDanger(Message) (Game|GetGameMode)))
  (if (and _notindanger (Math|Random|RandomBoolwithWeight (Variables|Default|GetBeginOverlapChance)))
    (if (!= (Utilities|Array|Length (Variables|Default|GetSpawnActors)) 0)
      (Utilities|FlowControl|DoOnce false
        (:Completed
          (Default|CallOnTriggered)
          (CallFunction|DarkCameraEffect)
          (CallFunction|PlayCombatMusic)
          (Audio|PlaySound2D (Variables|Default|GetTriggerSound) 1.0 1.0 0.0 0 0)
          (for _array_element (Variables|Default|GetSpawnActors)
            (for _index (range 0 (Math|Random|RandomIntegerinRange (- (Variables|Default|GetMinCount) 1) (- (Variables|Default|GetMaxCount) 1)))
              (bind _returnvalue (Game|SpawnActorfromClass (Variables|Default|GetClass) (Transformation|GetActorTransform _array_element) "AdjustIfPossibleButDontSpawnIfColliding" 0 "/Game/Sounds/Footsteps/Footsteps.Footsteps" 0))
              (if (Utilities|IsValid _returnvalue)
                (Default|SeePawn _returnvalue (Game|Player|GetPlayerPawn 0))))))))))

(event OnComponentEndOverlap(Box)
  (params (OverlappedComponent :type Primitive%20Component%20Object%20Reference) (OtherActor :type Actor%20Object%20Reference) (OtherComp :type Primitive%20Component%20Object%20Reference) (OtherBodyIndex :type Integer))
  (Utilities|Casting|CastToBP_PlayerCharacter OtherActor)
  (bind _notindanger (Class|GameModeInterface|GetPlayerinDanger(Message) (Game|GetGameMode)))
  (if (and _notindanger (Math|Random|RandomBoolwithWeight (Variables|Default|GetEndOverlapChance)))
    (if (!= (Utilities|Array|Length (Variables|Default|GetSpawnActors)) 0)
      (Utilities|FlowControl|DoOnce false
        (:Completed
          (Default|CallOnTriggered)
          (CallFunction|DarkCameraEffect)
          (CallFunction|PlayCombatMusic)
          (Audio|PlaySound2D (Variables|Default|GetTriggerSound) 1.0 1.0 0.0 0 0)
          (for _array_element (Variables|Default|GetSpawnActors)
            (for _index (range 0 (Math|Random|RandomIntegerinRange (- (Variables|Default|GetMinCount) 1) (- (Variables|Default|GetMaxCount) 1)))
              (bind _returnvalue (Game|SpawnActorfromClass (Variables|Default|GetClass) (Transformation|GetActorTransform _array_element) "AdjustIfPossibleButDontSpawnIfColliding" 0 "/Game/Sounds/Footsteps/Footsteps.Footsteps" 0))
              (if (Utilities|IsValid _returnvalue)
                (Default|SeePawn _returnvalue (Game|Player|GetPlayerPawn 0))))))))))

(event EventBeginPlay)

(event Collision|EventActorBeginOverlap
  (params (OtherActor :type Actor%20Object%20Reference)))

(event EventTick
  (params (DeltaSeconds :type Float%20%28single-precision%29)))

(fn ConstructionScript
  (Components|Box|SetBoxExtent (Variables|Default|GetBox) (Variables|Default|GetBoxExtent) true))

(fn DarkCameraEffect
  (if (Variables|Default|GetNeedDarkCameraEffect)
    (Class|PlayerCharacterInrerface|DarkCameraStart(Message) (Game|Player|GetPlayerPawn 0))
    (return)
    (else
      (return))))

(fn PlayCombatMusic
  (if (Variables|Default|GetNeedPlayCombatMusic)
    (Class|GameModeInterface|PlayCombatMusic(Message) (Game|GetGameMode))
    (return)
    (else
      (return))))