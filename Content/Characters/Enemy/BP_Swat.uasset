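; Rifle-armed SWAT enemy Blueprint that shoots at the player and becomes a lootable body when its mesh physics turns on.
; Animation notifies fire a randomly spread line trace toward the blackboard's player position, spawning surface-based impact effects, applying damage and writing back whether the player was hit.
; On death the weapon detaches and simulates physics.
; Inspection highlights body and weapon via custom depth, and interacting grants a grenade or magazine.
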(event EventTurnonMeshPhysics
  ;[1 1 1] InteractOn
  (|CallParentFunction)
  (Variables|Default|SetbCanInteract true))

(event EventEndInspection
  ;[1 1 1] EndInspection
  (Rendering|SetRenderCustomDepth (Variables|Character|GetMesh) false))

(event EventSetAimon
  ;[1 1 1] AimOn
  (Variables|Default|SetIsAiming true))

(event EventSetAimOff
  ;[1 1 1] AimOff
  (Variables|Default|SetIsAiming false))

(event EventOnNotifyBegin
  (params (NotifyName :type Name :default "None"))
  (bind _returnvalue (AI|GetBlackboard 0))
  (bind _returnvalue_2 (Transformation|GetActorLocation))
  (bind _returnvalue_3 (+ _returnvalue_2 "0, 0,50.000000"))
  ;[1 1 1] Attack
  (|CallParentFunction NotifyName)
  (Utilities|IsValid _returnvalue
    (:Is%20Valid
      (Audio|PlaySoundatLocation "/Game/Sounds/Weapon/SC_Weapon_Shot.SC_Weapon_Shot" _returnvalue_2 "0, 0, 0" 1.0 1.0 0.0 "/Game/Sounds/StandartSoundAttenuation.StandartSoundAttenuation" 0 0)
      (CallFunction|SpawnEmitters)
      (bind (_outhit _returnvalue_4) (Collision|LineTraceByChannel _returnvalue_3 (+ (+ _returnvalue_3 (* (Math|Vector|Normalize (- (+ (AI|Components|Blackboard|GetValueasVector _returnvalue (Variables|Default|GetPlayerPosition)) "0, 0,50.000000") _returnvalue_3)) 5e+03)) (Math|Vector|MakeVector (Math|Random|RandomFloatinRange -2.5e+02 2.5e+02) (Math|Random|RandomFloatinRange -2.5e+02 2.5e+02) (Math|Random|RandomFloatinRange -2.5e+02 2.5e+02))) "TraceTypeQuery3" false 0 "None"))
      (if _returnvalue_4
        (Effects|SpawnEmitterAttached (.Emitter (CallFunction|GetEmitterbyPhysMat (.physmat _outhit))) (.hitcomponent _outhit) "None" (.location _outhit) (Math|Conversions|RotationFromXVector (.normal _outhit)) (.EmitterScale (CallFunction|GetEmitterbyPhysMat (.physmat _outhit))) "KeepWorldPosition")
        (Audio|PlaySoundatLocation (.Sound (CallFunction|GetEmitterbyPhysMat (.physmat _outhit))) (.location _outhit) "0, 0, 0" 1.0 1.0 0.0 "/Game/Sounds/StandartSoundAttenuation.StandartSoundAttenuation" 0 0)
        (bind _isdamaged (CallFunction|DamageActor (.hitactor _outhit)))
        (if _isdamaged
          _
          (else
            _))
        (AI|Components|Blackboard|SetValueasBool (AI|GetBlackboard 0) (Variables|Default|GetIsPlayerHit) _isdamaged)
        (else
          (AI|Components|Blackboard|SetValueasBool (AI|GetBlackboard 0) (Variables|Default|GetIsPlayerHit) false))))))

(fn ConstructionScript
  (|CallParentFunction))

(fn CollisionSettingsonDeath
  (bind _weapon (Variables|Default|GetWeapon))
  (|CallParentFunction)
  (Collision|SetCollisionProfileName _weapon "CharacterMesh" true :!class /Script/Engine.PrimitiveComponent)
  (Transformation|DetachFromComponent _weapon "KeepWorld" "KeepWorld" "KeepWorld" true)
  (Variables|/Script/Engine.PrimitiveComponent|SetbGenerateOverlapEvents _weapon true)
  (Physics|SetSimulatePhysics _weapon true)
  (Collision|SetCollisionEnabled _weapon "QueryAndPhysics"))

(fn SpawnEmitters
  (Effects|SpawnEmitterAttached "/Game/Effects/Particles/P_Rifle_Muzzleflash.P_Rifle_Muzzleflash" (Variables|Default|GetWeapon) "MuzzleSocket" "0, 0, 0" "0, 0, 0" "1.000000,1.000000,1.000000" "SnapToTarget")
  (Effects|SpawnEmitterAttached "/Game/Effects/Particles/P_Rifle_ShellEject.P_Rifle_ShellEject" (Variables|Default|GetWeapon) "ShellEjectionSocket" "0, 0, 0" "0, 0, 0" "1.000000,1.000000,1.000000" "SnapToTarget")
  (return))

(fn BeginInspection
  (bind _bdropgrenade (Variables|Default|GetbDropGrenade))
  (Rendering|SetRenderCustomDepth (Variables|Character|GetMesh) true)
  (return (select _bdropgrenade "/Game/UI/Textures/T_Grenade.T_Grenade" "/Game/UI/Textures/T_Magazine.T_Magazine") (select _bdropgrenade "Grenade" "Ammo")))

(fn CanInteract
  (return (Variables|Default|GetbCanInteract)))

(fn StartInteract
  (params (Player :type BP%20Player%20Character%20Object%20Reference))
  (Default|PickUpEffect Player)
  (Audio|PlaySound2D "/Game/Sounds/Pickups/SC_Pickup.SC_Pickup" 1.0 1.0 0.0 0 0)
  (Variables|Default|SetbCanInteract false)
  (Rendering|SetRenderCustomDepth (Variables|Character|GetMesh) false)
  (if (Variables|Default|GetbDropGrenade)
    (bind _result (Math|Integer|IncrementInt (Variables|/Game/Characters/Player/BP_PlayerCharacter.BP_PlayerCharacter_C|GetGrenades Player))
      (:%20%20
        (Default|CallOnLaunchGrenade Player _result)
        (Variables|Default|SetEmpty true)
        (return true)))
    (else
      (bind _result_2 (Math|Integer|IncrementInt (Variables|/Game/Characters/Player/BP_PlayerCharacter.BP_PlayerCharacter_C|GetMagazines Player))
        (:%20%20
          (Default|CallOnMagazineChange Player _result_2)
          (Variables|Default|SetEmpty true)
          (return true))))))