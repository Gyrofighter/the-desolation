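; Game mode that plays the intro level sequence and directs background music for basic, combat, boss and ending states.
; Skipping stops a playing intro and starts basic music, otherwise it opens the HUD pause menu.
; Music crossfades set IsPlayerInDanger, with a DangerTime timer returning combat to a randomly chosen basic track.
; Boss music lengthens DangerTime, and GetPlayerInDanger returns the inverse of the danger flag.
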(event Custom|SkipIntro
  ;[1 1 1] SkipIntro
  (if (Audio|Components|Audio|IsPlaying (Variables|Default|GetIntroSequence))
    (Sequencer|Player|Stop (Variables|Default|GetIntroSequence) :!class /Script/MovieScene.MovieSceneSequencePlayer)
    (CallFunction|OnFinishedIntro)
    (else
      (bind _asbp_hud (Utilities|Casting|CastToBP_HUD (HUD|GetHUD (Game|GetPlayerController 0))))
      (Default|ShowPauseMenu _asbp_hud "Pause"))))

(event Custom|OnFinishedIntro
  ;[1 1 1] IntroFinished
  (Default|CallIntroFinished)
  (CallFunction|FadeinBasicMusic))

(event EventBeginPlay
  ;[1 1 1] BeginPlay
  (bind _returnvalue (Sequencer|Player|CreateLevelSequencePlayer (Variables|Default|GetIntroSequance)))
  (bind _output_get (Variables|Default|SetIntroSequence _returnvalue))
  (Sequencer|Player|Play _output_get :!class /Script/MovieScene.MovieSceneSequencePlayer)
  (EventDispatchers|AssignOnFinished _output_get (EventDispatchers|CreateEvent :!event Custom|OnFinishedIntro)))

(event EventPlayCombatMusic
  ;[1 1 1] CombatMusic
  (CallFunction|FadeinCombatMusic))

(event EventPlayBasicMusic
  ;[1 1 1] BasicMusic
  (if (not (Audio|Components|Audio|IsPlaying (Variables|Default|GetBasicMusic)))
    (CallFunction|FadeinBasicMusic)))

(event EventPlayBossMusic
  ;[1 1 1] BossMusic
  (Variables|Default|SetDangerTime 6e+02)
  (CallFunction|FadeinCombatMusic))

(event EventPlayEndMusic
  ;[1 1 1] EndMusic
  (Audio|Components|Audio|Stop (Variables|Default|GetCombatMusic))
  (Audio|PlaySound2D "/Game/Sounds/Music/InGame/SC_Music_Positive.SC_Music_Positive" 1.0 1.0 0.0 0 0))

(event EventSetPlayerSafe
  ;[1 1 1] PlayerSafe
  (Variables|Default|SetIsPlayerInDanger false))

(fn ConstructionScript)

(fn FadeinBasicMusic
  (Audio|Components|Audio|FadeOut (Variables|Default|GetCombatMusic) 3.0 0.0 "Linear" :!class /Script/Engine.AudioComponent)
  (Audio|Components|Audio|SetSound (Variables|Default|GetBasicMusic) (select (Math|Random|RandomBool) "/Game/Sounds/Music/InGame/SC_Music_HighIntensity.SC_Music_HighIntensity" "/Game/Sounds/Music/InGame/SC_Music_MediumIntensity.SC_Music_MediumIntensity"))
  (Audio|Components|Audio|FadeIn (Variables|Default|GetBasicMusic) 3.0 1.0 0.0 "Linear" :!class /Script/Engine.AudioComponent)
  (Variables|Default|SetIsPlayerInDanger false)
  (return))

(fn FadeinCombatMusic
  (Audio|Components|Audio|FadeOut (Variables|Default|GetBasicMusic) 3.0 0.0 "Linear" :!class /Script/Engine.AudioComponent)
  (Audio|Components|Audio|FadeIn (Variables|Default|GetCombatMusic) 3.0 1.0 0.0 "Linear" :!class /Script/Engine.AudioComponent)
  (Utilities|Time|SetTimerbyFunctionName 0 "FadeInBasicMusic" (Variables|Default|GetDangerTime))
  (Variables|Default|SetIsPlayerInDanger true)
  (return))

(fn GetPlayerinDanger
  (return (not (Variables|Default|GetIsPlayerInDanger))))