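; Base AI character that senses, chases and fights pawns of other factions, with random attack and hit montages.
; Sight, noise or damage sets the nearest living enemy as blackboard target, switches to run speed and pauses sensing until reset.
; Attack completion and hit reactions send StopAttack to the AI brain, with an immunity timer throttling hit montages.
; Death stops AI logic and capsule collision; notify and interrupt events are empty hooks.
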(event OnDeath(BP_HealthComponent)
  ;[1 1 1] Death
  (CallFunction|Death)
  (AI|Logic|StopLogic (Variables|/Script/AIModule.AIController|GetBrainComponent (AI|GetAIController self)) "")
  (bind _soundonseeenemycom (Variables|Default|GetSoundOnSeeEnemyCom)
    (:then
      (Audio|Components|Audio|FadeOut _soundonseeenemycom 0.5 0.0 "Linear" :!class /Script/Engine.AudioComponent))
    (:else)))

(event OnSeePawn(PawnSensing)
  (params (Pawn :type Pawn%20Object%20Reference))
  ;[1 1 1] SeePawn
  (CallFunction|SeePawn Pawn))

(event OnHearNoise(PawnSensing)
  (params (Instigator :type Pawn%20Object%20Reference) (Location :type Vector%20%28by%20ref%29 :default "0, 0, 0") (Volume :type Float%20%28single-precision%29))
  ;[1 1 1] SeePawn
  (CallFunction|SeePawn Instigator))

(event Custom|Death
  ;[1 1 1] Death
  (CallFunction|CollisionSettingsonDeath))

(event Custom|OnNotifyBegin
  (params (NotifyName :type Name))
  ;[1 1 1] Attack
)

(event Custom|OnNotifyEnd
  (params (NotifyName :type Name))
  ;[1 1 1] Attack
)

(event Custom|AttackInterrupted
  ;[1 1 1] Attack
)

(event Custom|CanPlayHitMontageAgain
  ;[1 1 1] AnyDamage
  (Variables|Default|SetCanPlayHitMontage true))

(event EventBeginPlay
  ;[1 1 1] BeginPlay
  (Variables|/Script/Engine.CharacterMovementComponent|SetMaxWalkSpeed (Variables|Character|GetCharacterMovement) (Variables|Default|GetWalkSpeed))
  (Variables|Default|SetStartLocation (Transformation|GetActorLocation)))

(event EventTurnonMeshPhysics
  ;[1 1 1] MeshPhysics
  (Physics|SetSimulatePhysics (Variables|Character|GetMesh) true)
  (Pawn|UnPossess (AI|GetAIController self)))

(event EventStartAttack
  ;[1 1 1] Attack
  (bind _returnvalue (Animation|GetCurrentMontage :!class /Script/Engine.Character))
  (if (or (Variables|Default|GetCanAttackFromHitMontage) (not (Utilities|Array|ContainsItem (Variables|Default|GetHitMontages) _returnvalue)))
    (bind _notifyname (Animation|Montage|PlayMontage (Variables|Character|GetMesh) (CallFunction|GetAttackMontage))
      (:OnCompleted
        (Class|AIBlueprintHelperLibrary|SendAIMessage self "StopAttack" 0 true)
        (Class|PawnNoiseEmitterComponent|MakeNoise (Variables|Default|GetPawnNoiseEmitter) self 1.0 (Transformation|GetActorLocation)))
      (:OnInterrupted
        (CallFunction|AttackInterrupted :!label _label))
      (:OnNotifyBegin
        (CallFunction|OnNotifyBegin _notifyname))
      (:OnNotifyEnd
        (CallFunction|OnNotifyEnd _notifyname)))
    (else
      (goto _label))))

(event EventResetSeePawns
  (bind _pawnsensing (Variables|Default|GetPawnSensing))
  ;[1 1 1] ResetSee
  (Variables|/Script/AIModule.PawnSensingComponent|SetbSeePawns _pawnsensing true)
  (Variables|/Script/AIModule.PawnSensingComponent|SetbHearNoises _pawnsensing true)
  (Variables|/Script/Engine.CharacterMovementComponent|SetMaxWalkSpeed (Variables|Character|GetCharacterMovement) (Variables|Default|GetWalkSpeed))
  (Variables|Default|SetTarget 0))

(event Game|Damage|EventAnyDamage
  (params (Damage :type Float%20%28single-precision%29) (DamageType :type Damage%20Type%20Object%20Reference) (InstigatedBy :type Controller%20Object%20Reference) (DamageCauser :type Actor%20Object%20Reference))
  ;[1 1 1] AnyDamage
  (if (not (Default|GetIsDead (Variables|Default|GetBP_HealthComponent)))
    (CallFunction|SeePawn DamageCauser)
    (if (Variables|Default|GetCanPlayHitMontage)
      (Variables|Default|SetCanPlayHitMontage false)
      (Animation|Montage|PlayMontage (Variables|Character|GetMesh) (CallFunction|GetHitMontage) (Math|Random|RandomFloatinRange 1.0 1.2)
        (:then
          (Utilities|Time|SetTimerbyFunctionName 0 "CanPlayHitMontageAgain" (Variables|Default|GetImmunityTime))
          (Class|AIBlueprintHelperLibrary|SendAIMessage self "StopAttack" 0 true))))))

(fn ConstructionScript
  (|CallParentFunction))

(fn GetAttackMontage
  (bind _attackmontages (Variables|Default|GetAttackMontages))
  (return (Utilities|Array|Get(acopy) _attackmontages (Math|Random|RandomInteger (Utilities|Array|Length _attackmontages)))))

(fn SeePawn
  (params (Actor :type Actor%20Object%20Reference))
  (bind _pawnsensing (Variables|Default|GetPawnSensing))
  (bind _fraction (Class|CharacterInterface|GetFraction(Message) Actor))
  (if (!= _fraction (Variables|Default|GetFraction))
    (bind _isdead (Class|CharacterInterface|IsDead(Message) Actor))
    (if (not _isdead)
      (Variables|Default|GetTarget
        (:then
          (if (< (Transformation|GetDistanceTo self Actor) (Transformation|GetDistanceTo self (Variables|Default|GetTarget)))
            (Variables|Default|SetTarget Actor :!label _label)
            (Variables|/Script/AIModule.PawnSensingComponent|SetbSeePawns _pawnsensing false)
            (Variables|/Script/AIModule.PawnSensingComponent|SetbHearNoises _pawnsensing false)
            (AI|Components|Blackboard|SetValueasObject (AI|GetBlackboard 0) (Variables|Default|GetBB_PlayerName) Actor)
            (Variables|/Script/Engine.CharacterMovementComponent|SetMaxWalkSpeed (Variables|Character|GetCharacterMovement) (Variables|Default|GetRunSpeed))
            (bind _soundonseeenemy (Variables|Default|GetSoundOnSeeEnemy)
              (:then
                (if (Math|Random|RandomBoolwithWeight (Variables|Default|GetChanceToCryWhenSeeEnemy))
                  (bind _returnvalue (Audio|SpawnSoundAttached _soundonseeenemy (Variables|Default|GetCapsuleComponent) "None" "0, 0, 0" "0, 0, 0" "SnapToTarget" true 1.0 1.0 0.0 0 0))
                  (Variables|Default|SetSoundOnSeeEnemyCom _returnvalue)))
              (:else))))
        (:else
          (goto _label))))))

(fn DamageActor
  (params (OtherActor :type Actor%20Object%20Reference))
  (bind _fraction (Class|CharacterInterface|GetFraction(Message) OtherActor))
  (if (and (!= _fraction (Variables|Default|GetFraction)) (Utilities|DoesObjectImplementInterface OtherActor "/Game/Base/CharacterInterface.CharacterInterface_C"))
    (Game|Damage|ApplyDamage OtherActor (CallFunction|GetDamage) (Pawn|GetController) self)
    (return true)
    (else
      (return false))))

(fn GetHitMontage
  (bind _hitmontages (Variables|Default|GetHitMontages))
  (return (Utilities|Array|Get(acopy) _hitmontages (Math|Random|RandomInteger (Utilities|Array|Length _hitmontages)))))

(fn CollisionSettingsonDeath
  (Collision|SetCollisionEnabled (Variables|Character|GetMesh) "QueryAndPhysics")
  (Collision|SetCollisionEnabled (Variables|Default|GetCapsuleComponent) "NoCollision"))

(fn GetDamage
  (bind _damageperattack (Variables|Default|GetDamagePerAttack))
  (bind _returnvalue (* _damageperattack 0.1))
  (return (Math|Random|RandomFloatinRange (- (Variables|Default|GetDamagePerAttack) _returnvalue) (+ (Variables|Default|GetDamagePerAttack) _returnvalue))))

(fn GetBehaviorTree
  (return (Variables|Default|GetBehaviorTree)))

(fn GetStartLocation
  (return (Variables|Default|GetStartLocation)))