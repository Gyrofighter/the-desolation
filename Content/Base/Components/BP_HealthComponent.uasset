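; Actor component that gives its owner health, with damage, healing, regeneration, instant kill, death and revive.
; It can auto-bind to the owner's any-damage event, and clamps health changes before broadcasting the new value and percent.
; Reaching zero through damage or kill fires the death event and optionally destroys the owner.
; Regeneration runs on a configurable tick while alive and below maximum, and revive restores full health.
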(event Custom|OnTakeAnyDamageByOwner
  (params (DamagedActor :type Actor%20Object%20Reference) (Damage :type Float%20%28single-precision%29) (DamageType :type Damage%20Type%20Object%20Reference) (InstigatedBy :type Controller%20Object%20Reference) (DamageCauser :type Actor%20Object%20Reference))
  ;[1 1 1] BeginPlay Assign On Take Damage
  (Health|TakeDamage Damage))

(event EventTick
  (params (DeltaSeconds :type Float%20%28single-precision%29))
  ;[1 1 1] EventTick Regeneration
  (if (Math|Boolean|ANDBoolean (> (Variables|Health|GetHealthPerSecond) 0.0) (not (Variables|System|GetIsDead)) (!= (Variables|Health|GetHealth) (Variables|Health|GetMaximumHealth)))
    (System|Regeneration DeltaSeconds)))

(event EventBeginPlay
  ;[1 1 1] BeginPlay Assign On Take Damage
  (Components|Tick|SetComponentTickEnabled (Variables|Performance|GetTickEnabled))
  (Class|ActorComponent|SetComponentTickInterval (Variables|Performance|GetTickInterval))
  (if (Variables|Settings|GetAssignOnTakeDamage)
    (EventDispatchers|AssignOnTakeAnyDamage (Components|GetOwner) (delegate Custom|OnTakeAnyDamageByOwner))))

(fn TakeDamage
  (params (Damage :type Float%20%28single-precision%29))
  (LocalVariables|SetL_HealthBeforeDamage (Variables|Health|GetHealth))
  (bind _output_get (Variables|Health|SetHealth (Math|Float|Clamp(Float) (- (Variables|Health|GetHealth) Damage) 0.0 (Variables|Health|GetMaximumHealth))))
  (if (!= _output_get (LocalVariables|GetL_HealthBeforeDamage))
    (Default|CallOnHealthChanged (Variables|Health|GetHealth) (/ (Variables|Health|GetHealth) (Variables|Health|GetMaximumHealth)))
    (if (== (Variables|Health|GetHealth) 0.0)
      (System|Death)
      (return)
      (else
        (return)))
    (else
      (return))))

(fn AddHealth
  (params (HealthToAdd :type Float%20%28single-precision%29))
  (LocalVariables|SetL_HealthBeforeAdd (Variables|Health|GetHealth))
  (bind _output_get (Variables|Health|SetHealth (Math|Float|Clamp(Float) (+ (Variables|Health|GetHealth) HealthToAdd) 0.0 (Variables|Health|GetMaximumHealth))))
  (if (!= _output_get (LocalVariables|GetL_HealthBeforeAdd))
    (Default|CallOnHealthChanged (Variables|Health|GetHealth) (/ (Variables|Health|GetHealth) (Variables|Health|GetMaximumHealth)))
    (if (== (Variables|Health|GetHealth) 0.0)
      (System|Death)
      (return)
      (else
        (return)))
    (else
      (return))))

(fn InstantKill
  (if (not (Variables|System|GetIsDead))
    (Variables|Health|SetHealth 0.0)
    (Default|CallOnHealthChanged 0.0 0.0)
    (System|Death)))

(fn Revive
  (if (Variables|System|GetIsDead)
    (Variables|System|SetIsDead false)
    (bind _output_get (Variables|Health|SetHealth (Variables|Health|GetMaximumHealth)))
    (Default|CallOnHealthChanged _output_get 1.0)
    (Default|CallOnRevive)
    (return)
    (else
      (return))))

(fn Death
  (Variables|System|SetIsDead true)
  (Default|CallOnDeath)
  (if (Variables|Settings|GetDestroyActorOnDeath)
    (Actor|DestroyActor (Components|GetOwner))))

(fn GetIsDead
  (return (Variables|System|GetIsDead)))

(fn Regeneration
  (params (DeltaSeconds :type Float%20%28single-precision%29))
  (bind _output_get (Variables|Health|SetHealth (Math|Float|Min(Float) (+ (* DeltaSeconds (Variables|Health|GetHealthPerSecond)) (Variables|Health|GetHealth)) (Variables|Health|GetMaximumHealth))))
  (Default|CallOnHealthChanged _output_get (/ _output_get (Variables|Health|GetMaximumHealth)))
  (return))