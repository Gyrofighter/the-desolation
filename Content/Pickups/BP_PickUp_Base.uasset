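; Base pickup actor that can be inspected and collected by the player.
; Beginning inspection turns on the static mesh's custom depth rendering and returns an info texture and text, and ending inspection turns custom depth off.
; Interacting triggers the player's pickup effect, plays a 2D pickup sound and destroys the actor.
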(event EventBeginPlay)

(event Collision|EventActorBeginOverlap
  (params (OtherActor :type Actor%20Object%20Reference)))

(event EventTick
  (params (DeltaSeconds :type Float%20%28single-precision%29)))

(event EventEndInspection
  (Rendering|SetRenderCustomDepth (Variables|Default|GetStaticMesh) false))

(event EventStartInteract
  (params (Player :type BP%20Player%20Character%20Object%20Reference))
  (Default|PickUpEffect Player)
  (Audio|PlaySound2D (Variables|Default|GetPickupSound) 1.0 1.0 0.0 0 0)
  (Actor|DestroyActor))

(fn ConstructionScript)

(fn BeginInspection
  (Rendering|SetRenderCustomDepth (Variables|Default|GetStaticMesh) true)
  (return (Variables|Default|GetInfoTexture) (Variables|Default|GetInfoText)))