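; BP_PickUp_AidKit is a health pickup that heals the interacting player.
; StartInteract checks the player's health component against a hard-coded near-100 threshold.
; Below it, the kit plays pickup feedback, adds AidKitHP, calls ActivateSpawner with ChanceToSpawn, destroys itself and returns true.
; Otherwise it shows a "Full" HUD message with a denied sound and returns false, leaving the kit in place.
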(fn ConstructionScript
  (|CallParentFunction))

(fn StartInteract
  (params (Player :type BP%20Player%20Character%20Object%20Reference))
  (bind _output_get (Variables|Default|SetPlayer Player))
  (if (< (Variables|/Game/Base/Components/BP_HealthComponent.BP_HealthComponent_C|GetHealth (Variables|/Game/Base/BP_BaseCharacter.BP_BaseCharacter_C|GetBP_HealthComponent Player)) 99.900002)
    (Default|PickUpEffect (Variables|Default|GetPlayer))
    (Audio|PlaySound2D (Variables|Default|GetPickupSound) 1.0 1.0 0.0 0 0)
    (Default|AddHealth (Variables|/Game/Base/BP_BaseCharacter.BP_BaseCharacter_C|GetBP_HealthComponent (Variables|Default|GetPlayer)) (Variables|Default|GetAidKitHP))
    (CallFunction|ActivateSpawner (Variables|Default|GetChanceToSpawn))
    (Actor|DestroyActor)
    (return true)
    (else
      (Class|HUDInterface|ShowInteractInfo(Message) (Default|GetHUD _output_get) (Variables|Default|GetInfoTexture) "Full")
      (Audio|PlaySound2D "/Game/Sounds/UI/SC_UI_Denied.SC_UI_Denied" 1.0 1.0 0.0 0 0)
      (return false))))